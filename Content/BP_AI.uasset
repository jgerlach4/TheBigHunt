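; BP_AI is a pawn that carries a BP_Animal child actor and patrols a looping list of waypoints.
; On BeginPlay it caches its first child actor as the animal and starts FollowWaypoint.
; FollowWaypoint issues AIMoveTo inside a while loop conditioned on the animal's IsDead being true.
; Each successful move advances the waypoint index, wraps it to zero at the end and calls FollowWaypoint again.
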(event Custom|Follow%20Waypoint
  (while (Variables|/Game/Blueprints/Animals/BP_Animal.BP_Animal_C|GetisDead (Variables|Default|GetAnimal))
    (AI|AIMoveTo self "0, 0, 0" (Utilities|Array|Get(acopy) (Variables|Default|Getwaypoint) (Variables|Default|GetcurrentWaypoint)) 1e+02 false
      (:OnSuccess
        (Math|Integer|IncrementInt (Variables|Default|GetcurrentWaypoint)
          (:%20%20
            (if (>= (Variables|Default|GetcurrentWaypoint) (Utilities|Array|Length (Variables|Default|Getwaypoint)))
              (Variables|Default|SetcurrentWaypoint 0))
            (CallFunction|FollowWaypoint)))))))

(event EventBeginPlay
  (bind _asbp_animal (Utilities|Casting|CastToBP_Animal (Utilities|Array|Get(acopy) (Actor|GetAllChildActors true))))
  (Variables|Default|SetAnimal _asbp_animal)
  (CallFunction|FollowWaypoint))

(event Collision|EventActorBeginOverlap
  (params (OtherActor :type Actor%20Object%20Reference)))

(event EventTick
  (params (DeltaSeconds :type Float%20%28single-precision%29)))

(fn ConstructionScript)