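; BP_Animal is a shootable animal that wanders between waypoints and awards points when killed.
; It loops through AIMoveTo waypoint walks, with weighted-random pauses for random idle animations, and only idles when it has no waypoints.
; Overlapping BP_Bullet actors subtract damage from health and are destroyed.
; On death it adds points through BP_Scorekeeper, plays a death animation and stops its movement.
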(event EventBeginPlay
  (if (not (Variables|Default|GetisDead)) :!label _label
    (if (or (== (Utilities|Array|Length (Variables|Default|GetWaypoint)) 0) (Math|Random|RandomBoolwithWeight (Variables|Default|GetwaypointPauseProbably)))
      ;[0.15 0.15 0.15 0.5] Idle animations
      (bind _output_get (Variables|Default|SetcurrentIdleAnimation (.OutItem (Utilities|Array|Random (Variables|Default|GetIdleAnimations)))))
      (Components|Animation|PlayAnimation (Variables|Default|GetSkeletalMesh) _output_get false)
      (Utilities|FlowControl|Delay (Animation|GetPlayLength _output_get))
      (goto _label)
      (else
        (Components|Animation|PlayAnimation (Variables|Default|GetSkeletalMesh) (Variables|Default|GetWalkAnimation) true)
        (AI|AIMoveTo self "0, 0, 0" (Utilities|Array|Get(acopy) (Variables|Default|Getwaypoint) (Variables|Default|GetcurrentWaypoint)) 5.0 false
          (:OnSuccess
            _)
          (:OnFail
            _))
        (Variables|Default|SetCurrentWaypoint (Math|Integer|%(Integer) (+ (Variables|Default|GetcurrentWaypoint) 1) (Utilities|Array|Length (Variables|Default|Getwaypoint))))
        (goto _label)))))

(event Collision|EventActorBeginOverlap
  (params (OtherActor :type Actor%20Object%20Reference))
  (if (not (Variables|Default|GetisDead))
    (bind _asbp_bullet (Utilities|Casting|CastToBP_Bullet OtherActor))
    (Variables|Default|SetHealth (- (Variables|Default|GetHealth) (Variables|/Game/Blueprints/Weapons/BP_Bullet.BP_Bullet_C|GetDamage _asbp_bullet)))
    (Actor|DestroyActor _asbp_bullet)
    (Development|PrintString (Utilities|String|ToString(Integer) (- (Variables|Default|GetHealth) (Variables|/Game/Blueprints/Weapons/BP_Bullet.BP_Bullet_C|GetDamage _asbp_bullet))))
    (if (<= (- (Variables|Default|GetHealth) (Variables|/Game/Blueprints/Weapons/BP_Bullet.BP_Bullet_C|GetDamage _asbp_bullet)) 0)
      (Development|PrintString "Dead")
      (bind _outactors (Actor|GetAllActorsOfClass "/Game/Blueprints/BP_Scorekeeper.BP_Scorekeeper_C"))
      (Default|AddPoints _outactors (Variables|Default|GetPointsValue))
      (Variables|Default|SetisDead true)
      (Components|Animation|PlayAnimation (Variables|Default|GetSkeletalMesh) (Variables|Default|GetDeathAnimation) false)
      (Components|Movement|StopMovementImmediately (Variables|Character|GetCharacterMovement)))))

(event EventTick
  (params (DeltaSeconds :type Float%20%28single-precision%29)))

(fn ConstructionScript)